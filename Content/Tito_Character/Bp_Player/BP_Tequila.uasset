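; BP_Tequila is a tequila pickup that the Tito player drinks on touch.
; Overlapping its sphere calls DrinkTequila on BP_TITOPlayer, then hides the mesh and disables collision.
; ResetTequila restores both after a delay, whose Duration grows by one second with each pickup, so every respawn takes longer.
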(event `Reset Tequila`
  (`KismetSystemLibrary.Delay` (`self.Duration`))
  (`SceneComponent.SetVisibility` (`self.StaticMesh`) true false)
  (`PrimitiveComponent.SetCollisionEnabled` (`self.Sphere`) "QueryOnly"))

(event `self.Sphere.OnComponentBeginOverlap`
  (params (OverlappedComponent :type "PrimitiveComponent Object Reference") (OtherActor :type "Actor Object Reference") (OtherComp :type "PrimitiveComponent Object Reference") (OtherBodyIndex :type Integer) (bFromSweep :type Boolean) (SweepResult :type "HitResult Structure (by ref)"))
  (bind _asbp_titoplayer (cast `/Game/Tito_Character/Bp_Player/BP_TITOPlayer` OtherActor))
  (`/Game/Tito_Character/Bp_Player/BP_TITOPlayer.Drink Tequila` _asbp_titoplayer)
  (`SceneComponent.SetVisibility` (`self.StaticMesh`) false false)
  (`PrimitiveComponent.SetCollisionEnabled` (`self.Sphere`) "NoCollision")
  (set `self.Duration` (+ (`self.Duration`) 1.0))
  (`self.Reset Tequila`))

(fn `UserConstructionScript`)