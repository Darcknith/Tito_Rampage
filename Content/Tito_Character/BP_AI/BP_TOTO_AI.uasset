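; AI brawler character that, once the player enters a fight, alternates random wandering with punching attacks.
; A BP_SpiderNet spawned and attached at BeginPlay picks each target, which AIMoveTo approaches before a punch montage and sphere trace damage other BP_TOTO_AI.
; Damage is gated during hit reactions, swaps eye expressions through a dynamic material, and at zero life disables movement and hitbox.
; Physical animation, tequila-level and input-mapping logic appear as unconnected leftovers.
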(event `Damage`
  (params (Damage :type Integer))
  (bind _charactermovement (`self.CharacterMovement`))
  (`/Engine/EditorBlueprintResources/StandardMacros.DoOnce` false :!label _label
    (:`Completed`
      (bind _output_get (set `self.Life` (`KismetMathLibrary.Clamp` (- (`self.Life`) Damage) 0 6)))
      (if (== _output_get 0)
        (`self.Ded Eye`)
        (`self.StopAnimMontage` (`self.GetCurrentMontage`))
        (`CharacterMovementComponent.DisableMovement` (`self.CharacterMovement`))
        (`|PlayMontage` (`self.Mesh`) "/Game/Tito_Character/Chara/animation/Tito_ded_Montage.Tito_ded_Montage" 0.7
          (:`then`
            (`PrimitiveComponent.SetCollisionEnabled` (`self.HitBox`) "NoCollision")
            (set `self.is dead` true)))
        (else
          (`self.StopAnimMontage` (`self.GetCurrentMontage`))
          (set `self.Can be select ?` false)
          (`self.OUCH Eye`)
          (`CharacterMovementComponent.DisableMovement` _charactermovement)
          (`|PlayMontage` (`self.Mesh`) "/Game/Tito_Character/Chara/animation/Tito_Hito_Montage.Tito_Hito_Montage" 1.2
            (:`OnCompleted`
              (`self.Classic Eye`)
              (`CharacterMovementComponent.SetMovementMode` _charactermovement "MOVE_Walking" 0)
              (`self.Move Random`)
              (`KismetSystemLibrary.Delay` 1.0)
              (set `self.Can be select ?` true)
              (goto _label :!via `Reset`))))))))

(event `ATK`
  ;[1 1 1] ATK
  (`|PlayMontage` (`self.Mesh`) (`|GetArrayItem` (`self.Punch Array`) (`self.Current Index`))
    (:`then`
      (`self.Trace Sphere`)
      (set `self.Current Index` (+ (`self.Current Index`) 1)))
    (:`OnCompleted`
      (set `self.Current Index` 0)
      (`self.Move Random`))))

(event `self.ReceiveBeginPlay`
  ;[0.05098 0.05098 0.05098] Event Begin Play
  (`self.set Eyes Mat`)
  (bind _returnvalue (`|SpawnActorFromClass` "/Game/Tito_Character/BP_AI/BP_SpiderNet.BP_SpiderNet_C" (`self.GetTransform`) "Undefined" "MultiplyWithRoot" null self (`self.Actor Select`) null))
  (`self.K2_AttachToActor` _returnvalue self (`self.Body Name`) "KeepWorld" "KeepWorld" "KeepWorld" true)
  (set `self.TargetNet` _returnvalue))

(event `Ded Eye`
  ;[1 1 1] Eye Change
  (`MaterialInstanceDynamic.SetScalarParameterValue` (`self.eye_mat`) "index" -1.0))

(event `self.ReceiveTick`
  (params (DeltaSeconds :type "Float (single-precision)"))
  (bind _asbp_titoplayer (cast `/Game/Tito_Character/Bp_Player/BP_TITOPlayer` (`GameplayStatics.GetPlayerCharacter` 0)))
  (bind _output_get (set `self.Is in Fight` (`/Game/Tito_Character/Bp_Player/BP_TITOPlayer.Is In Fight` _asbp_titoplayer)))
  (if _output_get
    (`/Engine/EditorBlueprintResources/StandardMacros.DoOnce` false
      (:`Completed`
        (`self.Move Random`)))))

(event `OUCH Eye`
  ;[1 1 1] Eye Change
  (`MaterialInstanceDynamic.SetScalarParameterValue` (`self.eye_mat`) "index" 1.0))

(event `Classic Eye`
  ;[1 1 1] Eye Change
  (`MaterialInstanceDynamic.SetScalarParameterValue` (`self.eye_mat`) "index" 0.0)
  (`MaterialInstanceDynamic.SetScalarParameterValue` (`self.eye_mat`) "offset" (`KismetMathLibrary.RandomFloatInRange` -1.0 1.5)))

(event `Find Target`
  (bind _targetnet (`self.TargetNet`)
    (:`then`
      (bind _target (`/Game/Tito_Character/BP_AI/BP_SpiderNet.Switch Target` _targetnet self (`self.Target`)))
      (set `self.Target` _target)
      (`|AIMoveTo` self (0.0 0.0 0.0) _target 150.0
        (:`OnSuccess`
          (`self.ATK`))))
    (:`else`)))

(event `Move Random`
  (bind _charactermovement (`self.CharacterMovement`))
  (`|AIMoveTo` self (`NavigationSystemV1.K2_GetRandomReachablePointInRadius` (`self.K2_GetActorLocation`) 1000.0 null null) null 150.0
    (:`then`
      (set `CharacterMovementComponent.MaxWalkSpeed` 200.0 _charactermovement))
    (:`OnSuccess`
      (set `CharacterMovementComponent.MaxWalkSpeed` 500.0 _charactermovement :!label _label_2)
      (if (`self.Is in Fight`)
        (`self.Find Target`)
        (else
          (`self.Move Random`))))
    (:`OnFail`
      (goto _label_2))))

(fn `set Eyes Mat`
  (bind _returnvalue (`PrimitiveComponent.CreateDynamicMaterialInstance` (`self.Mesh`) 1 (`PrimitiveComponent.GetMaterial` (`self.Mesh`) 1) "eyes"))
  (set `self.eye_mat` _returnvalue)
  (`self.Classic Eye`))

(fn `Set Physical Anim`
  (params (`Is Local Simulation` :type Boolean))
  (bind _body_name (`self.Body Name`))
  (bind _physicalanimation (`self.PhysicalAnimation`))
  (bind _mesh (`self.Mesh`))
  (`PhysicalAnimationComponent.SetSkeletalMeshComponent` _physicalanimation _mesh)
  (`PhysicalAnimationComponent.ApplyPhysicalAnimationSettingsBelow` _physicalanimation _body_name (make `PhysicalAnimationData` `Is Local Simulation` 1000.0 100.0 1000.0) true)
  (`SkeletalMeshComponent.SetAllBodiesBelowSimulatePhysics` _mesh _body_name true true))

(fn `Trace Sphere`
  (bind _returnvalue (`self.K2_GetActorLocation`))
  (bind _outhit (`KismetSystemLibrary.SphereTraceSingle` :`Start` _returnvalue :`End` (+ _returnvalue (* (`self.GetActorForwardVector`) 125.0)) :`Radius` 50.0 :`TraceChannel` "TraceTypeQuery1" :`DrawTime` 2.0))
  (bind (_bblockinghit _binitialoverlap _time _distance _location _impactpoint _normal _impactnormal _physmat _hitactor) (`GameplayStatics.BreakHitResult` _outhit))
  (if (`KismetSystemLibrary.DoesImplementInterface` _hitactor "/Game/Tito_Character/BPI_Fight.BPI_Fight_C")
    (bind _asbp_toto_ai (cast `/Game/Tito_Character/BP_AI/BP_TOTO_AI` _hitactor))
    (`self.Damage` _asbp_toto_ai 1)
    (return)))

(fn `UserConstructionScript`)