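; BP_SpiderNet is a targeting helper Blueprint that finds and picks nearby actors implementing BPI_Fight.
; Its functions gather candidates overlapping a Sphere, excluding an ignored or owning actor and the current or previous target.
; GetClosest and SwitchTarget choose by distance to that excluded actor, while SelectActor stores the choice.
; A RecentlyTargeted list separates fresh candidates, and debug prints show selected and closest actors.
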(fn `Get Closest`
  (params (Actors :type "Array of Actor Object Reference"))
  (returns (`Actor Select` :type "Actor Object Reference") (Disatance :type "Float (double-precision)"))
  (locals (`Closest Distance` :type "Float (double-precision)" :default 100000.0) (`Closest Actor` :type "Actor Object Reference"))
  (for _array_element Actors
    (bind _returnvalue (`self.GetDistanceTo` _array_element (`self.Actor To Ignor`)))
    (if (< _returnvalue (`local.Closest Distance`))
      (set `local.Closest Distance` _returnvalue)
      (bind _output_get (set `local.Closest Actor` _array_element))
      (`KismetSystemLibrary.PrintString` (`KismetSystemLibrary.GetDisplayName` _output_get))))
  (return (`local.Closest Actor`) (`local.Closest Distance`)))

(fn `Get Target In range`
  (returns (`Actor In Range` :type "Array of Actor Object Reference"))
  (bind _fresh_target_in_range (`self.Fresh Target In Range`))
  (for _array_element (`PrimitiveComponent.GetOverlappingActors` (`self.Sphere`) "/Script/Engine.Actor")
    (if (`KismetSystemLibrary.DoesImplementInterface` _array_element "/Game/Tito_Character/BPI_Fight.BPI_Fight_C")
      (if (and (!= (`self.Actor To Ignor`) _array_element) (!= (`self.Select Target`) _array_element))
        (`KismetArrayLibrary.Array_AddUnique` (`self.Actor In Range`) _array_element)
        (if (not (`KismetArrayLibrary.Array_Contains` (`self.Recently Targeted`) _array_element))
          (`KismetArrayLibrary.Array_AddUnique` (`self.Fresh Target In Range`) _array_element)))))
  (if (not (`KismetArrayLibrary.Array_IsEmpty` _fresh_target_in_range))
    (`KismetArrayLibrary.Array_Clear` (`self.Recently Targeted`))
    (return (`self.Actor In Range`))
    (else
      (return _fresh_target_in_range))))

(fn `Select Actor`
  (params (`Select Target` :type "Actor Object Reference"))
  (bind _output_get (set `self.Select Target` `Select Target`))
  (`KismetSystemLibrary.PrintString` (`KismetSystemLibrary.GetDisplayName` _output_get)))

(fn `Switch Target`
  (params (Owner :type "Actor Object Reference") (`Last One` :type "Actor Object Reference"))
  (returns (Target :type "Actor Object Reference"))
  (locals (`Last Target` :type "Actor Object Reference") (Distance :type "Float (double-precision)" :default 100000.0) (Target :type "Actor Object Reference"))
  (bind _actor_in_range (`self.Actor In Range`))
  (bind _last_one (`local.Last One`))
  (for _array_element (`PrimitiveComponent.GetOverlappingActors` (`self.Sphere`) "/Script/Engine.Actor")
    (if (`KismetSystemLibrary.DoesImplementInterface` _array_element "/Game/Tito_Character/BPI_Fight.BPI_Fight_C")
      (if (!= _array_element (`local.Owner`))
        (`KismetArrayLibrary.Array_Add` (`self.Actor In Range`) _array_element))))
  (if (`KismetArrayLibrary.Array_Contains` _actor_in_range _last_one)
    (`KismetArrayLibrary.Array_RemoveItem` _actor_in_range _last_one))
  (for _array_element_2 (`self.Actor In Range`)
    (bind _returnvalue (`self.GetDistanceTo` _array_element_2 (`local.Owner`)))
    (if (< _returnvalue (`local.Distance`))
      (if (not (== _array_element_2 (`local.Last One`)))
        (set `local.Distance` _returnvalue)
        (set `local.Last Target` _array_element_2))))
  (return (`local.Last Target`)))

(fn `UserConstructionScript`)