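; BP_Bottle_generator is a prop generator that builds a randomized row of bottles in its construction script.
; For each of NbBottle bottles, it adds an instance to one of four instanced mesh components picked at random.
; Local X is a random spacing multiplied by the index, with slight Y jitter, random yaw and random per-axis scale capped by variables.
; The event graph holds no active logic.
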(fn `UserConstructionScript`
  (bind _returnvalue (`KismetMathLibrary.RandomFloatInRange` 0.8 (`self.max_x/y scale`)))
  (set `self.Target` (`|MakeArray` (`self.bottle`) (`self.bottle1`) (`self.bottle2`) (`self.bottle3`)))
  (for _index (range (`self.nb_bottle`))
    (bind _returnvalue_2 (`InstancedStaticMeshComponent.AddInstance` (`KismetArrayLibrary.Array_Random` (`self.Target`)) (`KismetMathLibrary.MakeTransform` (`KismetMathLibrary.MakeVector` (* (`KismetMathLibrary.RandomFloatInRange` (`self.Min`) (`self.Max`)) _index) (`KismetMathLibrary.RandomFloatInRange` -3.0 3.0)) (`KismetMathLibrary.MakeRotator` 0.0 0.0 (`KismetMathLibrary.RandomFloatInRange` -90.0 90.0)) (`KismetMathLibrary.MakeVector` _returnvalue _returnvalue (`KismetMathLibrary.RandomFloatInRange` 0.6 (`self.max_hight`)))) false))))